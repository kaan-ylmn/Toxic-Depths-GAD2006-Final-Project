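; BP_Elevator is an elevator actor that rises and brings up the victory screen once triggered through OnElevatorReady.
; It stores its location at BeginPlay, then the ElevatorRise timeline lerps it 500 units upward without sweep.
; WBP_Victory is created and added to the viewport both when the timeline finishes and from a parallel fixed-delay branch, so two copies can appear.
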(event EventBeginPlay
  (Variables|Default|SetStartLocation (Transformation|GetActorLocation)))

(event Collision|EventActorBeginOverlap
  (params (OtherActor :type Actor%20Object%20Reference)))

(event EventTick
  (params (DeltaSeconds :type Float%20%28single-precision%29)))

(event EventOnElevatorReady
  (bind _startlocation (Variables|Default|GetStartLocation))
  (Utilities|FlowControl|Sequence
    (:then_0
      (bind _alpha (Timeline|ElevatorRise PlayFromStart)
        (:Update
          (Transformation|SetActorLocation (Math|Vector|Lerp(Vector) _startlocation (+ _startlocation (Math|Vector|MakeVector 0.0 0.0 5e+02)) _alpha) false false))
        (:Finished
          (Development|PrintString "FINISHED CALISTI")
          (bind _returnvalue (UserInterface|CreateWidget "/Game/WBP_Victory.WBP_Victory_C"))
          (UserInterface|Viewport|AddtoViewport _returnvalue 0))))
    (:then_1
      (Development|PrintString "FINISHED CALISTI")
      (Utilities|FlowControl|Delay 3.1)
      (bind _returnvalue_2 (UserInterface|CreateWidget "/Game/WBP_Victory.WBP_Victory_C"))
      (UserInterface|Viewport|AddtoViewport _returnvalue_2 0))))

(fn ConstructionScript)